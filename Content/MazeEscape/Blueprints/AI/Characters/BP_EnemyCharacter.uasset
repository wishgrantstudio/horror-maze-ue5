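; Maze enemy character that patrols between two points, chases the player on sight and triggers the loss on contact.
; PawnSensing sightings store the player's location, raise walk speed and start an AIMoveTo chase.
; A looping timer drops the chase whenever the player is beyond close range, searching the last seen location before resuming patrol after a random pause.
; Capsule hits against the player call PlayerLost on BP_GameMode.
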(event `self.ReceiveBeginPlay`
  (`KismetSystemLibrary.K2_SetTimerDelegate` (delegate `CheckPlayerVisibility`) 0.3 true)
  (set `self.bMovingToA` true)
  (`self.MoveToPatrolPoint`))

(event `CheckPlayerVisibility`
  ; Chasing Player?
  (if (`self.bIsChasing`)
    (if (> (`self.GetDistanceTo` (`self.LastSeenPlayer`)) 100.0)
      (set `self.bIsChasing` false)
      (set `CharacterMovementComponent.MaxWalkSpeed` 200.0 (`self.CharacterMovement`))
      (set `self.Searching` true)
      (`|AIMoveTo` self (`self.LastSeenLocation`) null 100.0
        (:`OnSuccess`
          (`KismetSystemLibrary.Delay` (`KismetMathLibrary.RandomFloatInRange` 1.0 3.0))
          (if (`self.Searching`)
            (set `self.Searching` false)
            (if (or (`self.Searching`) (`self.bMovingToA`))
              (`|AIMoveTo` self (0.0 0.0 0.0) (`self.PatrolPointA`)
                (:`OnSuccess`
                  (`self.MoveToPatrolPoint`)))
              (else
                (`|AIMoveTo` self (0.0 0.0 0.0) (`self.PatrolPointB`)
                  (:`OnSuccess`
                    (`self.MoveToPatrolPoint`)))))))))))

(event `MoveToPatrolPoint`
  ; Patrol Point Loop
  (`KismetSystemLibrary.Delay` 1.0)
  (if (`self.bIsChasing`)
    _
    (elif (`self.bMovingToA`)
      (set `self.bMovingToA` false)
      (`|AIMoveTo` self (0.0 0.0 0.0) (`self.PatrolPointB`)
        (:`OnSuccess`
          (`self.MoveToPatrolPoint`)))
      (else
        (set `self.bMovingToA` true)
        (`|AIMoveTo` self (0.0 0.0 0.0) (`self.PatrolPointA`)
          (:`OnSuccess`
            (`self.MoveToPatrolPoint`)))))))

(event `self.PawnSensing.OnSeePawn`
  (params (Pawn :type "Pawn Object Reference"))
  ; i see player
  (bind _asbp_player_charector (cast `/Game/MazeEscape/Blueprints/Characters/BP_PlayerCharector` Pawn))
  (bind _output_get (set `self.LastSeenPlayer` _asbp_player_charector))
  (set `self.LastSeenLocation` (`self.K2_GetActorLocation` _output_get))
  (set `self.Searching` false)
  (set `self.bIsChasing` true)
  (set `CharacterMovementComponent.MaxWalkSpeed` 3000.0 (`self.CharacterMovement`))
  (`|AIMoveTo` self (0.0 0.0 0.0) _output_get))

(event `self.CapsuleComponent.OnComponentHit`
  (params (HitComponent :type "PrimitiveComponent Object Reference") (OtherActor :type "Actor Object Reference") (OtherComp :type "PrimitiveComponent Object Reference") (NormalImpulse :type "Vector Structure") (Hit :type "HitResult Structure (by ref)"))
  ;[0.15 0.05045 0.04141 0.5] Losing Condition
  (cast `/Game/MazeEscape/Blueprints/Characters/BP_PlayerCharector` OtherActor)
  (bind _asbp_game_mode (cast `/Game/MazeEscape/Blueprints/Game/BP_GameMode` (`GameplayStatics.GetGameMode`)))
  (`/Game/MazeEscape/Blueprints/Game/BP_GameMode.PlayerLost` _asbp_game_mode))

(fn `UserConstructionScript`)
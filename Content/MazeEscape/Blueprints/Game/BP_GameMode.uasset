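; Game mode for the maze escape game that runs the countdown, plays cave sound and handles win or loss.
; A looping one-second timer decrements TimeRemaining and refreshes BP_PlayerController's HUD, with GetFormattedTime supplying minutes-and-seconds text.
; PlayerWon and PlayerLost pause, stop the timer and show end widgets with UI-only input.
; Timeout calls UILost directly without pausing; its timer clear names no function and GameOver is empty.
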(event `self.ReceiveBeginPlay`
  (set `self.TimeRemaining` (`self.GameDuration`))
  (bind _returnvalue (`KismetSystemLibrary.K2_SetTimerDelegate` (delegate `TimerTicker`) 1.0 true))
  (set `self.GameTimerHandle` _returnvalue)
  (`AudioComponent.Play` (`self.CaveSound`) 0.0))

(event `TimerTicker`
  (`self.UpdateTimer`))

(event `UILost`
  ;[0.15 0.07551 0.06769 0.5] UI LOST
  (bind _returnvalue (`InputDeviceLibrary.GetPlayerControllerFromPlatformUser` (struct)))
  (bind _asbp_player_controller (cast `/Game/MazeEscape/Blueprints/Game/BP_PlayerController` _returnvalue))
  (`Controller.SetIgnoreMoveInput` _asbp_player_controller true)
  (`Controller.SetIgnoreLookInput` _asbp_player_controller true)
  (bind _returnvalue_2 (`|CreateWidget` "/Game/MazeEscape/Blueprints/UI/WBP_Defeat.WBP_Defeat_C"))
  (`UserWidget.AddToViewport` _returnvalue_2 0)
  (set `PlayerController.bShowMouseCursor` true _asbp_player_controller)
  (`WidgetBlueprintLibrary.SetInputMode_UIOnlyEx` _asbp_player_controller null))

(event `UIWin`
  ;[0.09557 0.15 0.08176 0.5] UI WIN
  (bind _returnvalue (`InputDeviceLibrary.GetPlayerControllerFromPlatformUser` (struct)))
  (bind _asbp_player_controller (cast `/Game/MazeEscape/Blueprints/Game/BP_PlayerController` _returnvalue))
  (`Controller.SetIgnoreMoveInput` _asbp_player_controller true)
  (`Controller.SetIgnoreLookInput` _asbp_player_controller true)
  (bind _returnvalue_2 (`|CreateWidget` "/Game/MazeEscape/Blueprints/UI/WBP_Win.WBP_Win_C"))
  (`UserWidget.AddToViewport` _returnvalue_2 0)
  (set `PlayerController.bShowMouseCursor` true _asbp_player_controller)
  (`WidgetBlueprintLibrary.SetInputMode_UIOnlyEx` _asbp_player_controller null))

(fn `GameOver`)

(fn `GetFormattedTime`
  (returns (return :type Text))
  (bind _timeremaining (`self.TimeRemaining`))
  (return (`|FormatText` "{Min} : {Sec}" (`KismetTextLibrary.Conv_IntToText` (/ _timeremaining 60) false true 2) (`KismetTextLibrary.Conv_IntToText` (mod _timeremaining 60) false true 2))))

(fn `PlayerLost`
  (if (not (`self.GameEnded`))
    (`GameplayStatics.SetGamePaused` true)
    (`KismetSystemLibrary.PrintString` "Player Lost")
    (bind _returnvalue (`InputDeviceLibrary.GetPlayerControllerFromPlatformUser` (struct)))
    (`Controller.SetIgnoreLookInput` _returnvalue true)
    (`Controller.SetIgnoreMoveInput` _returnvalue true)
    (set `self.GameEnded` true)
    (`KismetSystemLibrary.K2_ClearAndInvalidateTimerHandle` (`self.GameTimerHandle`))
    (`self.UILost`)))

(fn `PlayerWon`
  (`GameplayStatics.SetGamePaused` true)
  (`KismetSystemLibrary.K2_ClearAndInvalidateTimerHandle` (`self.GameTimerHandle`))
  (bind _returnvalue (`InputDeviceLibrary.GetPlayerControllerFromPlatformUser` (struct)))
  (`Controller.SetIgnoreMoveInput` _returnvalue true)
  (`Controller.SetIgnoreLookInput` _returnvalue true)
  (`self.UIWin`))

(fn `UpdateTimer`
  (set `self.TimeRemaining` (- (`self.TimeRemaining`) 1.0))
  (bind _asbp_player_controller (cast `/Game/MazeEscape/Blueprints/Game/BP_PlayerController` (`GameplayStatics.GetPlayerController` 0)))
  (`/Game/MazeEscape/Blueprints/Game/BP_PlayerController.RefreshHUD` _asbp_player_controller)
  (if (<= (`self.TimeRemaining`) 0.0)
    (set `self.TimeRemaining` 0)
    (`KismetSystemLibrary.K2_ClearTimer` null)
    (`self.GameOver`)
    (`self.UILost`)))

(fn `UserConstructionScript`)